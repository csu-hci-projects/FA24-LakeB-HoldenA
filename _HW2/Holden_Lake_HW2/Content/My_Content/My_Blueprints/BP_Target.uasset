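; BP_Target is a shootable-style target actor that counts toward a level's remaining-target total.
; On BeginPlay it caches the LevelController and, if Moving, runs a Timeline that lerps it from its starting location toward TargetLocation.
; Each Hit event decrements Health, and a hit received at zero Health destroys the target and decrements the controller's TargetsLeft.
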(event `self.ReceiveBeginPlay`
  (bind _returnvalue (`GameplayStatics.GetActorOfClass` "/Game/My_Content/My_Blueprints/LevelController.LevelController_C"))
  (set `self.LevelController` _returnvalue)
  (if (`self.Moving`)
    (set `self.OGLocation` (`self.K2_GetActorLocation`))
    (bind (_direction _movement) (`Timeline|Timeline` :!via `PlayFromStart`)
      (:`Update`
        (`self.K2_SetActorLocation` (`KismetMathLibrary.VLerp` (`self.OGLocation`) (`self.TargetLocation`) _movement))))))

(event `self.ReceiveHit`
  (params (MyComp :type "PrimitiveComponent Object Reference") (Other :type "Actor Object Reference") (OtherComp :type "PrimitiveComponent Object Reference") (bSelfMoved :type Boolean) (HitLocation :type "Vector Structure") (HitNormal :type "Vector Structure") (NormalImpulse :type "Vector Structure") (Hit :type "HitResult Structure (by ref)"))
  (bind _levelcontroller (`self.LevelController`))
  (if (== (`self.Health`) 0)
    (`self.K2_DestroyActor`)
    (bind _result (`/Engine/EditorBlueprintResources/StandardMacros.DecrementInt` (`/Game/My_Content/My_Blueprints/LevelController.TargetsLeft` _levelcontroller))
      (:`  `
        (set `/Game/My_Content/My_Blueprints/LevelController.TargetsLeft` _result _levelcontroller)))
    (else
      (bind _result_2 (`/Engine/EditorBlueprintResources/StandardMacros.DecrementInt` (`self.Health`))
        (:`  `
          (set `self.Health` _result_2))))))

(fn `UserConstructionScript`)