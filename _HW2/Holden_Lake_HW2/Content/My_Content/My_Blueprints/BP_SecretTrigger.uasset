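; BP_SecretTrigger is a trigger actor that opens a secret wall when hit by an actor tagged KEY.
; On BeginPlay it finds a SecretWall actor by class, stores its location and computes a target position below it.
; A qualifying hit plays a timeline from the start, lerping the wall down to that target without sweep.
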(event `self.ReceiveBeginPlay`
  (bind _returnvalue (`GameplayStatics.GetActorOfClass` "/Game/My_Content/My_Blueprints/SecretWall.SecretWall_C"))
  (bind _output_get (set `self.ST_WallRef` _returnvalue))
  (bind _output_get_2 (set `self.ST_OGPosition` (`self.K2_GetActorLocation` _output_get)))
  (set `self.ST_TargetPosition` (+ _output_get_2 (0.0 0.0 -600.0))))

(event `self.ReceiveHit`
  (params (MyComp :type "PrimitiveComponent Object Reference") (Other :type "Actor Object Reference") (OtherComp :type "PrimitiveComponent Object Reference") (bSelfMoved :type Boolean) (HitLocation :type "Vector Structure") (HitNormal :type "Vector Structure") (NormalImpulse :type "Vector Structure") (Hit :type "HitResult Structure (by ref)"))
  (if (`self.ActorHasTag` Other "KEY")
    (bind (_direction _movement) (`Timeline|Timeline` :!via `PlayFromStart`)
      (:`Update`
        (`self.K2_SetActorLocation` (`self.ST_WallRef`) (`KismetMathLibrary.VLerp` (`self.ST_OGPosition`) (`self.ST_TargetPosition`) _movement) false false)))))

(fn `UserConstructionScript`)